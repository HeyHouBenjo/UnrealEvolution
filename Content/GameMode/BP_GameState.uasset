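; Game state Blueprint that populates a simulation with entities, food and poison at random positions.
; On BeginPlay it spawns a batch of BP_Entity actors and plays two timelines, whose Spawn event tracks are wired to add BP_Food and BP_Poison.
; Spawned food and poison are tracked in FoodItems and PoisonItems, with functions to remove them.
; Positions are random within a Size-bounded square at a fixed height.
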(event `self.ReceiveBeginPlay`
  (for _ (range 51)
    (`|SpawnActorFromClass` "/Game/Blueprints/BP_Entity.BP_Entity_C" (`KismetMathLibrary.MakeTransform` (`self.GetRandomPosition`)) "Undefined" "OverrideRootScale" null null))
  (`TimelineComponent.Play` (`self.T_SpawnFood`))
  (`TimelineComponent.Play` (`self.T_SpawnPoison`)))

(fn `GetRandomPosition`
  (returns (Position :type "Vector Structure"))
  (locals (size :type "Float (double-precision)" :default 2000.0))
  (bind _size (`local.size`))
  (bind _returnvalue (* _size -1.0))
  (return (`KismetMathLibrary.MakeVector` (`KismetMathLibrary.RandomFloatInRange` _returnvalue _size) (`KismetMathLibrary.RandomFloatInRange` _returnvalue _size) 100.0)))

(fn `RemoveFood`
  (params (food :type "/Game/Blueprints/BP_Food Object Reference"))
  (`KismetArrayLibrary.Array_RemoveItem` (`self.FoodItems`) food))

(fn `RemovePoison`
  (params (poison :type "/Game/Blueprints/BP_Poison Object Reference"))
  (`KismetArrayLibrary.Array_RemoveItem` (`self.PoisonItems`) poison))

(fn `SpawnFood`
  (params (location :type "Vector Structure"))
  (bind _returnvalue (`|SpawnActorFromClass` "/Game/Blueprints/BP_Food.BP_Food_C" (`KismetMathLibrary.MakeTransform` location) "Undefined" "OverrideRootScale" null null))
  (`KismetArrayLibrary.Array_Add` (`self.FoodItems`) _returnvalue))

(fn `SpawnPoison`
  (params (location :type "Vector Structure"))
  (bind _returnvalue (`|SpawnActorFromClass` "/Game/Blueprints/BP_Poison.BP_Poison_C" (`KismetMathLibrary.MakeTransform` location) "Undefined" "OverrideRootScale" null null))
  (`KismetArrayLibrary.Array_Add` (`self.PoisonItems`) _returnvalue))

(fn `UserConstructionScript`)