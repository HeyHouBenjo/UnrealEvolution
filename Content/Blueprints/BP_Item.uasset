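; BP_Item is the base pickup for BP_Food and BP_Poison, consumed by BP_Entity actors on overlap.
; A timeline with randomized length destroys the item when its lifetime ends.
; A DoOnce-gated overlap lerps the item to the entity, then calls the empty Consume hook and destroys it, resetting if the entity becomes invalid or dying.
; On destruction, food or poison removes itself from BP_GameState.
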(event `self.ReceiveDestroyed`
  (bind _asbp_game_state (cast `/Game/GameMode/BP_GameState` (`GameplayStatics.GetGameState`)))
  (bind _asbp_food (cast `/Game/Blueprints/BP_Food` self)
    (:`then`
      (`/Game/GameMode/BP_GameState.RemoveFood` _asbp_game_state _asbp_food))
    (:`CastFailed`
      (bind _asbp_poison (cast `/Game/Blueprints/BP_Poison` self))
      (`/Game/GameMode/BP_GameState.RemovePoison` _asbp_game_state _asbp_poison))))

(event `self.ReceiveBeginPlay`
  (`TimelineComponent.SetTimelineLength` (`self.DeathTimer`) (`KismetMathLibrary.RandomFloatInRange` 5.0 10.0))
  (`Timeline|DeathTimer`
    (:`Finished`
      (`self.K2_DestroyActor`))))

(event `self.Item.OnComponentBeginOverlap`
  (params (OverlappedComponent :type "PrimitiveComponent Object Reference") (OtherActor :type "Actor Object Reference") (OtherComp :type "PrimitiveComponent Object Reference") (OtherBodyIndex :type Integer) (bFromSweep :type Boolean) (SweepResult :type "HitResult Structure (by ref)"))
  (`/Engine/EditorBlueprintResources/StandardMacros.DoOnce` false :!label _label
    (:`Completed`
      (bind _asbp_entity (cast `/Game/Blueprints/BP_Entity` OtherActor)
        (:`then`
          (set `self.StartPos` (`self.K2_GetActorLocation`))
          (bind (_direction _moveprogress) (`Timeline|MoveToConsumer` :!via `PlayFromStart`)
            (:`Update`
              (`self.EntityIsValidAndLiving` _asbp_entity
                (:`True`
                  (`self.K2_SetActorLocation` (`KismetMathLibrary.VLerp` (`self.StartPos`) (`self.K2_GetActorLocation` _asbp_entity) _moveprogress)))
                (:`False`
                  (`TimelineComponent.Stop` (`self.MoveToConsumer`) :!label _label_2)
                  (goto _label :!via `Reset`))))
            (:`Finished`
              (`self.EntityIsValidAndLiving` _asbp_entity
                (:`True`
                  (`self.Consume` _asbp_entity)
                  (`self.K2_DestroyActor`))
                (:`False`
                  (goto _label_2))))))
        (:`CastFailed`
          (goto _label :!via `Reset`))))))

(fn `Consume`
  (params (CollectingEntity :type "/Game/Blueprints/BP_Entity Object Reference")))

(fn `UserConstructionScript`)