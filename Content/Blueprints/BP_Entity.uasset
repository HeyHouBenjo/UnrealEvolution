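; BP_Entity is a steering agent that seeks food and dodges poison while its health drains over time.
; Each tick it adds a pull toward the nearest GameState food and weighted poison avoidance to its clamped velocity, stopping when no food exists.
; Avoidance sums perpendicular turns away from poison ahead, scaled by facing and proximity.
; At zero health it plays a Die timeline meant to scale and destroy it; UpdateVisual is empty.
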(event `self.ReceiveBeginPlay`
  (bind _asbp_game_state (cast `/Game/GameMode/BP_GameState` (`GameplayStatics.GetGameState`)))
  (set `self.GameState` _asbp_game_state))

(event `self.ReceiveTick`
  (params (DeltaSeconds :type "Float (single-precision)"))
  (`self.MoveEntity` DeltaSeconds)
  (`self.DecayHealth` DeltaSeconds
    (:`Lives`
      _)
    (:`Dies`
      (`TimelineComponent.Play` (`self.Die`))))
  (`self.UpdateVisual`))

(fn `GetNearestFood`
  (params (FoodItems :type "Array of /Game/Blueprints/BP_Food Object Reference"))
  (returns (Food :type "/Game/Blueprints/BP_Food Object Reference") (Location :type "Vector Structure"))
  (locals (MinDistIndex :type Integer) (MinDist :type "Float (double-precision)" :default 5000.0))
  (bind _output (`|GetArrayItem` FoodItems (`local.MinDistIndex`)))
  (for (_array_element _array_index) FoodItems
    (bind _returnvalue (`self.GetDistanceTo` _array_element))
    (if (< _returnvalue (`local.MinDist`))
      (set `local.MinDist` _returnvalue)
      (set `local.MinDistIndex` _array_index)))
  (return _output (`self.K2_GetActorLocation` _output)))

(fn `GetNewVelocity`
  (returns (Velocity :type "Vector Structure"))
  (bind _gamestate (`self.GameState`))
  (bind _fooditems (`/Game/GameMode/BP_GameState.FoodItems` _gamestate))
  (`/Game/Libraries/BP_MacroLibrary.ArrayIsEmpty` _fooditems
    (:`IsEmpty`
      (return (0.0 0.0 0.0)))
    (:`IsNotEmpty`
      (return (`KismetMathLibrary.Vector_ClampSizeMax` (+ (* (+ (`self.VelocityFromFood` _fooditems) (* (`self.VelocityFromPoison` (`/Game/GameMode/BP_GameState.PoisonItems` _gamestate)) (`self.DodgeImportance`))) (* (`self.MaxVelocity`) (`self.Steering`))) (`self.CurrentVelocity`)) (`self.MaxVelocity`))))))

(fn `GetTurnVector`
  (params (DirToPoison :type "Vector Structure") (MoveDirection :type "Vector Structure") (Multiplier :type "Float (double-precision)"))
  (returns (ReturnValue :type "Vector Structure"))
  (bind _returnvalue (`KismetMathLibrary.MakeVector` (* -1 MoveDirection_Y) MoveDirection_X MoveDirection_Z))
  (bind _returnvalue_2 (* _returnvalue Multiplier))
  (if (< (`KismetMathLibrary.Dot_VectorVector` _returnvalue DirToPoison) 0.0)
    (return _returnvalue_2)
    (else
      (return (* _returnvalue_2 -1.0)))))

(fn `MoveEntity`
  (params (`Delta Seconds` :type "Float (double-precision)"))
  (bind _output_get (set `self.CurrentVelocity` (`self.GetNewVelocity`)))
  (`self.K2_AddActorWorldOffset` (* _output_get `Delta Seconds`)))

(fn `UpdateVisual`)

(fn `UserConstructionScript`)

(fn `VelocityFromFood`
  (params (FoodItems :type "Array of /Game/Blueprints/BP_Food Object Reference (by ref)"))
  (returns (Velocity :type "Vector Structure"))
  (return (`KismetMathLibrary.Normal` (- (`.Location` (`self.GetNearestFood` FoodItems)) (`self.K2_GetActorLocation`)))))

(fn `VelocityFromPoison`
  (params (PoisonItems :type "Array of /Game/Blueprints/BP_Poison Object Reference"))
  (returns (Velocity :type "Vector Structure"))
  (locals (AddedVelocities :type "Vector Structure"))
  (bind _maxvelocity (`self.MaxVelocity`))
  (bind _returnvalue (`KismetMathLibrary.Normal` (`self.CurrentVelocity`)))
  (for _array_element PoisonItems
    (bind _returnvalue_2 (`KismetMathLibrary.Normal` (- (`self.K2_GetActorLocation` _array_element) (`self.K2_GetActorLocation`))))
    (bind _returnvalue_3 (`KismetMathLibrary.Dot_VectorVector` _returnvalue_2 _returnvalue))
    (if (> _returnvalue_3 0.0)
      (set `local.AddedVelocities` (+ (`self.GetTurnVector` _returnvalue_2 _returnvalue (* _returnvalue_3 (- 1.0 (/ (`KismetMathLibrary.FClamp` (`self.GetDistanceTo` _array_element) 0.0 _maxvelocity) _maxvelocity)))) (`local.AddedVelocities`)))))
  (return (`KismetMathLibrary.ClampVectorSize` (`local.AddedVelocities`) 0.0 5.0)))